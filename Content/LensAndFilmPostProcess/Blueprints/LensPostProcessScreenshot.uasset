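; Post-process volume actor that applies toggleable lens and film effects: blur, chromatic aberration, distortion, sharpening, grain/grunge, color adjustment and light leaks.
; The construction script runs MainFunction, which creates and caches a dynamic material per enabled slot and pushes the exposed parameters into it.
; Grain/grunge and color/leaks each share a slot, picking a combined or single-effect material.
; It then assigns the blendables and applies box extent and volume settings.
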(event EventBeginPlay)

(event Collision|EventActorBeginOverlap
  (params (OtherActor :type Actor%20Object%20Reference)))

(event EventTick
  (params (DeltaSeconds :type Float%20%28single-precision%29)))

(fn ConstructionScript
  (CallFunction|MainFunction))

(fn MainFunction
  (bind _postprocess (Variables|Default|GetPostProcess))
  (bind _lightleaks (Variables|LightLeaks|GetLightLeaks))
  (bind _filmgrunge (Variables|FilmGrunge|GetFilmGrunge))
  (bind _graintexture (Variables|FilmGrain|GetGrainTexture))
  (bind _grungetexture (Variables|FilmGrunge|GetGrungeTexture))
  (bind _grungetexturescale (Variables|FilmGrunge|GetGrungeTextureScale))
  (Utilities|Array|Clear (Variables|Materials|GetPostProcessMaterials))
  (for (_array_element _array_index) (Utilities|Array|MakeArray (Variables|Blur|GetBlur) (Variables|ChromaticAberration|GetChromaticAberration) (Variables|LensDistortion|GetLensDistortion) (Variables|UnsharpMasking|GetUnsharpMasking) (or (Variables|FilmGrain|GetFilmGrain) (Variables|FilmGrunge|GetFilmGrunge)) (or (Variables|ColorAdjustment|GetColorAdjustment) (Variables|LightLeaks|GetLightLeaks)))
    (if _array_element
      (Utilities|IsValid (Utilities|Array|Get(acopy) (Variables|Default|GetDMI) _array_index)
        (:Is%20Valid
          _)
        (:Is%20Not%20Valid
          (bind _returnvalue (Rendering|Material|CreateDynamicMaterialInstance (Utilities|Array|Get(acopy) (Utilities|Array|MakeArray (Variables|Materials|GetBlurMaterial) (Variables|Materials|GetAberrationMaterial) (Variables|Materials|GetDistortionMaterial) (Variables|Materials|GetSharpenMaterial) (select (and _filmgrunge (Variables|FilmGrain|GetFilmGrain)) (Variables|Materials|GetFilmMaterialBoth) (select _filmgrunge (Variables|Materials|GetFilmMaterialGrunge) (Variables|Materials|GetFilmMaterialGrain))) (select (and _lightleaks (Variables|ColorAdjustment|GetColorAdjustment)) (Variables|Materials|GetColorAdjustmentWithLightLeaksMaterial) (select _lightleaks (Variables|Materials|GetLightLeaksMaterial) (Variables|Materials|GetColorAdjustmentMaterial)))) _array_index) "None" "None" :!class /Script/Engine.KismetMaterialLibrary))
          (Utilities|Array|SetArrayElem (Variables|Default|GetDMI) _array_index _returnvalue true)))
      (Utilities|Array|Add (Variables|Materials|GetPostProcessMaterials) (Utilities|Struct|MakeWeightedBlendable 1.0 (Utilities|Array|Get(acopy) (Variables|Default|GetDMI) _array_index)))
      (switch int _array_index
        (:0
          (Rendering|Material|SetScalarParameterValue (Utilities|Array|Get(acopy) (Variables|Default|GetDMI) _array_index) "BlurRadius" (Variables|Blur|GetBlurRadius) :!class /Script/Engine.MaterialInstanceDynamic)
          (Rendering|Material|SetScalarParameterValue (Utilities|Array|Get(acopy) (Variables|Default|GetDMI) _array_index) "BlurRadiusConstant" (Variables|Blur|GetBlurRadiusConstant) :!class /Script/Engine.MaterialInstanceDynamic)
          (Rendering|Material|SetScalarParameterValue (Utilities|Array|Get(acopy) (Variables|Default|GetDMI) _array_index) "BlurFadeExponent" (Variables|Blur|GetBlurFadeExponent) :!class /Script/Engine.MaterialInstanceDynamic)
          (Rendering|Material|SetScalarParameterValue (Utilities|Array|Get(acopy) (Variables|Default|GetDMI) _array_index) "BlurQuality" (Math|Conversions|ToFloat(Byte) (Variables|Blur|GetBlurQuality)) :!class /Script/Engine.MaterialInstanceDynamic))
        (:1
          (Rendering|Material|SetScalarParameterValue (Utilities|Array|Get(acopy) (Variables|Default|GetDMI) _array_index) "Red/Cyan" (Variables|ChromaticAberration|GetRed/Cyan) :!class /Script/Engine.MaterialInstanceDynamic)
          (Rendering|Material|SetScalarParameterValue (Utilities|Array|Get(acopy) (Variables|Default|GetDMI) _array_index) "Green/Magenta" (Variables|ChromaticAberration|GetGreen/Magenta) :!class /Script/Engine.MaterialInstanceDynamic)
          (Rendering|Material|SetScalarParameterValue (Utilities|Array|Get(acopy) (Variables|Default|GetDMI) _array_index) "Blue/Yellow" (Variables|ChromaticAberration|GetBlue/Yellow%20) :!class /Script/Engine.MaterialInstanceDynamic)
          (Rendering|Material|SetScalarParameterValue (Utilities|Array|Get(acopy) (Variables|Default|GetDMI) _array_index) "AberrationFadeExponent" (Variables|ChromaticAberration|GetAberrationFadeExponent) :!class /Script/Engine.MaterialInstanceDynamic))
        (:2
          (Rendering|Material|SetScalarParameterValue (Utilities|Array|Get(acopy) (Variables|Default|GetDMI) _array_index) "DistortionAmount" (Variables|LensDistortion|GetDistortionAmount) :!class /Script/Engine.MaterialInstanceDynamic))
        (:3
          (Rendering|Material|SetScalarParameterValue (Utilities|Array|Get(acopy) (Variables|Default|GetDMI) _array_index) "SharpenIntensity" (Variables|UnsharpMasking|GetSharpenIntensity) :!class /Script/Engine.MaterialInstanceDynamic)
          (Rendering|Material|SetScalarParameterValue (Utilities|Array|Get(acopy) (Variables|Default|GetDMI) _array_index) "Balance" (Variables|UnsharpMasking|GetBalance) :!class /Script/Engine.MaterialInstanceDynamic)
          (Rendering|Material|SetScalarParameterValue (Utilities|Array|Get(acopy) (Variables|Default|GetDMI) _array_index) "UnsharpBlurRadius" (Variables|UnsharpMasking|GetUnsharpBlurRadius) :!class /Script/Engine.MaterialInstanceDynamic)
          (Rendering|Material|SetScalarParameterValue (Utilities|Array|Get(acopy) (Variables|Default|GetDMI) _array_index) "UnsharpBlurQuality" (Math|Conversions|ToFloat(Byte) (Variables|UnsharpMasking|GetUnsharpBlurQuality)) :!class /Script/Engine.MaterialInstanceDynamic))
        (:4
          (Rendering|Material|SetScalarParameterValue (Utilities|Array|Get(acopy) (Variables|Default|GetDMI) _array_index) "GrainAmount" (Variables|FilmGrain|GetGrainAmount) :!class /Script/Engine.MaterialInstanceDynamic)
          (Rendering|Material|SetScalarParameterValue (Utilities|Array|Get(acopy) (Variables|Default|GetDMI) _array_index) "GrainScale" (Variables|FilmGrain|GetGrainScale) :!class /Script/Engine.MaterialInstanceDynamic)
          (Rendering|Material|SetScalarParameterValue (Utilities|Array|Get(acopy) (Variables|Default|GetDMI) _array_index) "GrainRate" (Variables|FilmGrain|GetGrainRate) :!class /Script/Engine.MaterialInstanceDynamic)
          (Rendering|Material|SetScalarParameterValue (Utilities|Array|Get(acopy) (Variables|Default|GetDMI) _array_index) "GrainDesaturation" (Variables|FilmGrain|GetGrainDesaturation) :!class /Script/Engine.MaterialInstanceDynamic)
          (Rendering|Material|SetTextureParameterValue (Utilities|Array|Get(acopy) (Variables|Default|GetDMI) _array_index) "GrainTexture" _graintexture)
          (Rendering|Material|SetScalarParameterValue (Utilities|Array|Get(acopy) (Variables|Default|GetDMI) _array_index) "GrainTextureX" (Math|Conversions|ToFloat(Integer) (Class|Texture2D|BlueprintGetSizeX _graintexture)) :!class /Script/Engine.MaterialInstanceDynamic)
          (Rendering|Material|SetScalarParameterValue (Utilities|Array|Get(acopy) (Variables|Default|GetDMI) _array_index) "GrainTextureY" (Math|Conversions|ToFloat(Integer) (Class|Texture2D|BlueprintGetSizeY _graintexture)) :!class /Script/Engine.MaterialInstanceDynamic)
          (Rendering|Material|SetScalarParameterValue (Utilities|Array|Get(acopy) (Variables|Default|GetDMI) _array_index) "ShadowsDesaturation" (Variables|FilmGrain|GetShadowsDesaturation) :!class /Script/Engine.MaterialInstanceDynamic)
          (Rendering|Material|SetScalarParameterValue (Utilities|Array|Get(acopy) (Variables|Default|GetDMI) _array_index) "ShadowsDesaturationThreshold" (Variables|FilmGrain|GetShadowsDesaturationThreshold) :!class /Script/Engine.MaterialInstanceDynamic)
          (Rendering|Material|SetScalarParameterValue (Utilities|Array|Get(acopy) (Variables|Default|GetDMI) _array_index) "ShadowsDesaturationNoise" (Variables|FilmGrain|GetShadowsDesaturationNoise) :!class /Script/Engine.MaterialInstanceDynamic)
          (Rendering|Material|SetScalarParameterValue (Utilities|Array|Get(acopy) (Variables|Default|GetDMI) _array_index) "GrungeDensity1" (Variables|FilmGrunge|GetGrungeDensity1) :!class /Script/Engine.MaterialInstanceDynamic)
          (Rendering|Material|SetScalarParameterValue (Utilities|Array|Get(acopy) (Variables|Default|GetDMI) _array_index) "GrungeDensity2" (Variables|FilmGrunge|GetGrungeDensity2) :!class /Script/Engine.MaterialInstanceDynamic)
          (Rendering|Material|SetScalarParameterValue (Utilities|Array|Get(acopy) (Variables|Default|GetDMI) _array_index) "GrungeFPS" (Variables|FilmGrunge|GetGrungeFPS) :!class /Script/Engine.MaterialInstanceDynamic)
          (Rendering|Material|SetTextureParameterValue (Utilities|Array|Get(acopy) (Variables|Default|GetDMI) _array_index) "GrungeTexture" _grungetexture)
          (Rendering|Material|SetScalarParameterValue (Utilities|Array|Get(acopy) (Variables|Default|GetDMI) _array_index) "GrungeTextureX" (* (Math|Conversions|ToFloat(Integer) (Class|Texture2D|BlueprintGetSizeX _grungetexture)) _grungetexturescale) :!class /Script/Engine.MaterialInstanceDynamic)
          (Rendering|Material|SetScalarParameterValue (Utilities|Array|Get(acopy) (Variables|Default|GetDMI) _array_index) "GrungeTextureY" (* (Math|Conversions|ToFloat(Integer) (Class|Texture2D|BlueprintGetSizeY _grungetexture)) _grungetexturescale) :!class /Script/Engine.MaterialInstanceDynamic))
        (:5
          (Rendering|Material|SetScalarParameterValue (Utilities|Array|Get(acopy) (Variables|Default|GetDMI) _array_index) "Reds" (Variables|ColorAdjustment|GetReds) :!class /Script/Engine.MaterialInstanceDynamic)
          (Rendering|Material|SetScalarParameterValue (Utilities|Array|Get(acopy) (Variables|Default|GetDMI) _array_index) "Yellows" (Variables|ColorAdjustment|GetYellows) :!class /Script/Engine.MaterialInstanceDynamic)
          (Rendering|Material|SetScalarParameterValue (Utilities|Array|Get(acopy) (Variables|Default|GetDMI) _array_index) "Greens" (Variables|ColorAdjustment|GetGreens) :!class /Script/Engine.MaterialInstanceDynamic)
          (Rendering|Material|SetScalarParameterValue (Utilities|Array|Get(acopy) (Variables|Default|GetDMI) _array_index) "Cyans" (Variables|ColorAdjustment|GetCyans) :!class /Script/Engine.MaterialInstanceDynamic)
          (Rendering|Material|SetScalarParameterValue (Utilities|Array|Get(acopy) (Variables|Default|GetDMI) _array_index) "Blues" (Variables|ColorAdjustment|GetBlues) :!class /Script/Engine.MaterialInstanceDynamic)
          (Rendering|Material|SetScalarParameterValue (Utilities|Array|Get(acopy) (Variables|Default|GetDMI) _array_index) "Magentas" (Variables|ColorAdjustment|GetMagentas) :!class /Script/Engine.MaterialInstanceDynamic)
          (Rendering|Material|SetScalarParameterValue (Utilities|Array|Get(acopy) (Variables|Default|GetDMI) _array_index) "BlackAndWhite" (Variables|ColorAdjustment|GetBlackAndWhite) :!class /Script/Engine.MaterialInstanceDynamic)
          (Rendering|Material|SetScalarParameterValue (Utilities|Array|Get(acopy) (Variables|Default|GetDMI) _array_index) "LIghtLeaksContrast" (Variables|LightLeaks|GetLIghtLeaksContrast) :!class /Script/Engine.MaterialInstanceDynamic)
          (Rendering|Material|SetScalarParameterValue (Utilities|Array|Get(acopy) (Variables|Default|GetDMI) _array_index) "LIghtLeaksFPS" (Variables|LightLeaks|GetLIghtLeaksFPS) :!class /Script/Engine.MaterialInstanceDynamic)
          (Rendering|Material|SetScalarParameterValue (Utilities|Array|Get(acopy) (Variables|Default|GetDMI) _array_index) "LIghtLeaksRate" (Variables|LightLeaks|GetLIghtLeaksRate) :!class /Script/Engine.MaterialInstanceDynamic)
          (Rendering|Material|SetVectorParameterValue (Utilities|Array|Get(acopy) (Variables|Default|GetDMI) _array_index) "LeaksColor1" (Variables|LightLeaks|GetLeaksColor1) :!class /Script/Engine.MaterialInstanceDynamic)
          (Rendering|Material|SetVectorParameterValue (Utilities|Array|Get(acopy) (Variables|Default|GetDMI) _array_index) "LeaksColor2" (Variables|LightLeaks|GetLeaksColor2) :!class /Script/Engine.MaterialInstanceDynamic)
          (Rendering|Material|SetVectorParameterValue (Utilities|Array|Get(acopy) (Variables|Default|GetDMI) _array_index) "LeaksColor3" (Variables|LightLeaks|GetLeaksColor3) :!class /Script/Engine.MaterialInstanceDynamic)))))
  (Utilities|Struct|SetmembersinPostProcessSettings (Variables|/Script/Engine.PostProcessComponent|GetSettings (Variables|Default|GetPostProcess)) (Utilities|Struct|MakeWeightedBlendables (Variables|Materials|GetPostProcessMaterials)))
  (Components|Box|SetBoxExtent (Variables|Default|GetBox) (Variables|General|GetVolumeExtent) true)
  (Variables|/Script/Engine.PostProcessComponent|SetbUnbound _postprocess (Variables|General|GetUnbound))
  (Variables|/Script/Engine.PostProcessComponent|SetbEnabled _postprocess (Variables|General|GetEnabled))
  (Variables|/Script/Engine.PostProcessComponent|SetPriority _postprocess (Variables|General|GetPriority))
  (Variables|/Script/Engine.PostProcessComponent|SetBlendRadius _postprocess (Variables|General|GetBlendRadius)))